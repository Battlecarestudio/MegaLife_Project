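; Destructible block for the bomb game that can drop power-up or power-down items when damaged.
; MC_Set_Destructible sets the replicated type, whose RepNotify picks the mesh, and plays a timeline that animates height and scale on spawn.
; On authority, Damage spawns a BombSpawner_BP at the block, then destroys it.
; Half the time it also drops a floating bomb, blast or speed item, weighted 2:1 toward upgrades.
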(event Custom|MC_Set_Destructible
  (params (Destructible_Type :type Destructible_Types%20Enum :default "NewEnumerator0"))
  ;[0.1979 0.1979 0.1979] Sets up this destructible with the incoming mesh and plays a nice spawning effect
  (Variables|Default|SetDestructible_Type Destructible_Type) ; Double click me
  (bind (_direction _location _scale) (Timeline|SpawnEffect PlayFromStart)
    (:Update
      (Transformation|SetRelativeTransform (Variables|Default|GetCube) (Math|Transform|MakeTransform (Math|Vector|MakeVector 0.0 0.0 _location) "0, 0, 0" (Math|Vector|MakeVector _scale _scale _scale)) false false))))

(event EventDamage
  (bind _returnvalue (Transformation|GetActorLocation))
  (bind _returnvalue_2 (+ (.z _returnvalue) 5e+01))
  (bind _returnvalue_3 (Math|Conversions|ToTransform(Vector) (Math|Vector|MakeVector (.x _returnvalue) (.y _returnvalue) _returnvalue_2)))
  ;[0.1979 0.1979 0.1979] Incase this destructible block gets destroyed, then randomly either an Item (powerup/down) gets spawned, or none get spawned at all > afterwards we destroy this actor
  (Networking|SwitchHasAuthority
    (:Authority
      (Game|SpawnActorfromClass "/Game/BomberGuys/Blueprints/Core/Gameplay/Actors/Spawners/BombSpawner_BP.BombSpawner_BP_C" (Math|Conversions|ToTransform(Vector) (Math|Vector|MakeVector (.x _returnvalue) (.y _returnvalue) (.z _returnvalue))) "AlwaysSpawn" 0 false 0)
      (switch int (Math|Random|RandomIntegerinRange 0 5) ; 50% chance that an item gets dropped
        (:0
          (CallFunction|SpawnBombItem _returnvalue_3))
        (:1
          (CallFunction|SpawnBlastItem _returnvalue_3))
        (:2
          (CallFunction|SpawnSpeedItem _returnvalue_3))
        (:3
          _)
        (:4
          _)
        (:5
          _))
      (Actor|DestroyActor))))

(fn ConstructionScript)

(fn SetMesh
  (params (Destructible_Type :type Destructible_Types%20Enum :default "NewEnumerator0"))
  ;[0.1979 0.1979 0.1979] Spawns the corresponding Mesh based on the incoming Destructible type
  (switch Utilities|FlowControl|Switch|SwitchonDestructible_Types Destructible_Type
    (:NewEnumerator0
      (Components|StaticMesh|SetStaticMesh (Variables|Default|GetCube) "/Game/BomberGuys/Assets/3D_Assets/Meshes/Blocks/Bricks_Destructible.Bricks_Destructible"))
    (:NewEnumerator1
      (Components|StaticMesh|SetStaticMesh (Variables|Default|GetCube) "/Game/BomberGuys/Assets/3D_Assets/Meshes/Blocks/Cone_Destructible.Cone_Destructible"))
    (:NewEnumerator2
      (Components|StaticMesh|SetStaticMesh (Variables|Default|GetCube) "/Game/BomberGuys/Assets/3D_Assets/Meshes/Blocks/MetalPipes_Destructible.MetalPipes_Destructible"))
    (:NewEnumerator3
      (Components|StaticMesh|SetStaticMesh (Variables|Default|GetCube) "/Game/BomberGuys/Assets/3D_Assets/Meshes/Blocks/MovingBox_Destructible.MovingBox_Destructible"))
    (:NewEnumerator4
      (Components|StaticMesh|SetStaticMesh (Variables|Default|GetCube) "/Game/BomberGuys/Assets/3D_Assets/Meshes/Blocks/NeonCube_Destructible.NeonCube_Destructible"))
    (:NewEnumerator5
      (Components|StaticMesh|SetStaticMesh (Variables|Default|GetCube) "/Game/BomberGuys/Assets/3D_Assets/Meshes/Blocks/TreeGreen_Destructible.TreeGreen_Destructible"))
    (:NewEnumerator6
      (Components|StaticMesh|SetStaticMesh (Variables|Default|GetCube) "/Game/BomberGuys/Assets/3D_Assets/Meshes/Blocks/TreeOrange_Destructible.TreeOrange_Destructible")))
  (return))

(fn SpawnBombItem
  (params (SpawnTransform :type Transform))
  (switch int (Math|Random|RandomIntegerinRange 0 2)
    (:0
      (Game|SpawnActorfromClass "/Game/BomberGuys/Blueprints/Core/Gameplay/Actors/Items/Item_BombUp.Item_BombUp_C" SpawnTransform "AlwaysSpawn" 0 0 :!label _label) ; 2/3 chance for a Bomb up item
    )
    (:1
      (goto _label))
    (:2
      (Game|SpawnActorfromClass "/Game/BomberGuys/Blueprints/Core/Gameplay/Actors/Items/Item_BombDown.Item_BombDown_C" SpawnTransform "AlwaysSpawn" 0 0) ; 1/3 chance for a Bomb down item
    ))
  (return))

(fn SpawnBlastItem
  (params (SpawnTransform :type Transform))
  (switch int (Math|Random|RandomIntegerinRange 0 2)
    (:0
      (Game|SpawnActorfromClass "/Game/BomberGuys/Blueprints/Core/Gameplay/Actors/Items/Item_BlastUp.Item_BlastUp_C" SpawnTransform "AlwaysSpawn" 0 0 :!label _label) ; 2/3 chance for a Blast up item
    )
    (:1
      (goto _label))
    (:2
      (Game|SpawnActorfromClass "/Game/BomberGuys/Blueprints/Core/Gameplay/Actors/Items/Item_BlastDown.Item_BlastDown_C" SpawnTransform "AlwaysSpawn" 0 0) ; 1/3 chance for a Blast down item
    ))
  (return))

(fn SpawnSpeedItem
  (params (SpawnTransform :type Transform))
  (switch int (Math|Random|RandomIntegerinRange 0 2)
    (:0
      (Game|SpawnActorfromClass "/Game/BomberGuys/Blueprints/Core/Gameplay/Actors/Items/Item_SpeedUp.Item_SpeedUp_C" SpawnTransform "AlwaysSpawn" 0 0 :!label _label) ; 2/3 chance for Speed up item
    )
    (:1
      (goto _label))
    (:2
      (Game|SpawnActorfromClass "/Game/BomberGuys/Blueprints/Core/Gameplay/Actors/Items/Item_SpeedDown.Item_SpeedDown_C" SpawnTransform "AlwaysSpawn" 0 0) ; 1/3 chance for Speed down item
    ))
  (return))

(fn OnRepDestructibleType
  (CallFunction|SetMesh (Variables|Default|GetDestructible_Type)))