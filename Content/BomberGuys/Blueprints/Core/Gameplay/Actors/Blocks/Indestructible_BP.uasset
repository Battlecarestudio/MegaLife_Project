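; Indestructible block actor for Bomber Guys that takes its look from an IndestructibleType, such as rock, books or tire stacks.
; MC_Set_Indestructible stores the type and plays a timeline that animates the mesh's height and uniform scale as a spawn effect.
; The type's RepNotify calls SetMesh, which swaps in the matching static mesh.
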(event Custom|MC_Set_Indestructible
  (params (Indestructible_Type :type Indestructible_Types%20Enum :default "NewEnumerator0"))
  ;[0.1979 0.1979 0.1979] Sets up this indestructible with the incoming mesh and plays a nice spawning effect
  (Variables|Default|SetIndestructible_Type Indestructible_Type)
  (bind (_direction _location _scale) (Timeline|SpawnEffect PlayFromStart)
    (:Update
      (Transformation|SetRelativeTransform (Variables|Default|GetCube) (Math|Transform|MakeTransform (Math|Vector|MakeVector 0.0 0.0 _location) "0, 0, 0" (Math|Vector|MakeVector _scale _scale _scale)) false false))))

(fn ConstructionScript)

(fn SetMesh
  (params (Indestructible_Type :type Indestructible_Types%20Enum :default "NewEnumerator0"))
  ;[0.1979 0.1979 0.1979] Spawns the corresponding Mesh based on the incoming Indestructible type
  (switch Utilities|FlowControl|Switch|SwitchonIndestructible_Types Indestructible_Type
    (:NewEnumerator0
      (Components|StaticMesh|SetStaticMesh (Variables|Default|GetCube) "/Game/BomberGuys/Assets/3D_Assets/Meshes/Blocks/MetalBlock_Indestructible.MetalBlock_Indestructible"))
    (:NewEnumerator1
      (Components|StaticMesh|SetStaticMesh (Variables|Default|GetCube) "/Game/BomberGuys/Assets/3D_Assets/Meshes/Blocks/TireStackTriple_Indestructible.TireStackTriple_Indestructible"))
    (:NewEnumerator6
      (Components|StaticMesh|SetStaticMesh (Variables|Default|GetCube) "/Game/BomberGuys/Assets/3D_Assets/Meshes/Blocks/TireStackDouble_Indestructible.TireStackDouble_Indestructible"))
    (:NewEnumerator2
      (Components|StaticMesh|SetStaticMesh (Variables|Default|GetCube) "/Game/BomberGuys/Assets/3D_Assets/Meshes/Blocks/ConstructionBlock_Indestructible.ConstructionBlock_Indestructible"))
    (:NewEnumerator3
      (Components|StaticMesh|SetStaticMesh (Variables|Default|GetCube) "/Game/BomberGuys/Assets/3D_Assets/Meshes/Blocks/Books_Indestructible.Books_Indestructible"))
    (:NewEnumerator4
      (Components|StaticMesh|SetStaticMesh (Variables|Default|GetCube) "/Game/BomberGuys/Assets/3D_Assets/Meshes/Blocks/NeonCube_Indestructible.NeonCube_Indestructible"))
    (:NewEnumerator5
      (Components|StaticMesh|SetStaticMesh (Variables|Default|GetCube) "/Game/BomberGuys/Assets/3D_Assets/Meshes/Blocks/Rock_Indestructible.Rock_Indestructible")))
  (return))

(fn OnRepIndestructibleType
  (CallFunction|SetMesh (Variables|Default|GetIndestructible_Type)))