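; ActorSpawner_BP is a map placement point that spawns either a destructible or a bomb spawner at its location when its Choose event runs.
; With MustBeBombSpawner set, it always spawns a bomb spawner so players at corner spawn points are not stuck.
; Otherwise it picks randomly with equal odds, passing DestructibleType to any new destructible.
; The construction script swaps the billboard sprite to mark forced spawn-point instances.
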(event Custom|Choose
  (bind _returnvalue (Transformation|GetActorLocation))
  (if (Variables|Default|GetMustBeBombSpawner?)
    ;[0.1979 0.1979 0.1979] Spawn a bomb spawner if we have selected that this actor must spawn one. Neccesary for the spawn points / corners of the map so that players can move on spawn and won't be stuck
    (Game|SpawnActorfromClass "/Game/BomberGuys/Blueprints/Core/Gameplay/Actors/Spawners/BombSpawner_BP.BombSpawner_BP_C" (Math|Transform|MakeTransform (Transformation|GetActorLocation) "0, 0, 0" "1,1,1") "Undefined" 0 false 0)
    (else
      ;[0.1979 0.1979 0.1979] Randomly spawns either a Destructible_BP or a BombSpawner_BP
      (if (== (Math|Random|RandomIntegerinRange 1 2) 1)
        (bind _returnvalue_2 (Game|SpawnActorfromClass "/Game/BomberGuys/Blueprints/Core/Gameplay/Actors/Blocks/Destructible_BP.Destructible_BP_C" (Math|Transform|MakeTransform _returnvalue "0, 0, 0" "1,1,1") "Undefined" 0 0))
        (Default|MCSetDestructible _returnvalue_2 (Variables|Default|GetDestructible_Type))
        (else
          (Game|SpawnActorfromClass "/Game/BomberGuys/Blueprints/Core/Gameplay/Actors/Spawners/BombSpawner_BP.BombSpawner_BP_C" (Math|Transform|MakeTransform _returnvalue "0, 0, 0" "1,1,1") "Undefined" 0 false 0))))))

(fn ConstructionScript
  (if (Variables|Default|GetMustBeBombSpawner?)
    (Rendering|Components|Sprite|SetSprite (Variables|Default|GetBillboard) "/Game/BomberGuys/Assets/3D_Assets/Textures/Actor_Billboard_Images/Billboard_ActorSpawner_Spawnpoint.Billboard_ActorSpawner_Spawnpoint")
    (else
      (Rendering|Components|Sprite|SetSprite (Variables|Default|GetBillboard) "/Game/BomberGuys/Assets/3D_Assets/Textures/Actor_Billboard_Images/Billboard_ActorSpawner.Billboard_ActorSpawner"))))