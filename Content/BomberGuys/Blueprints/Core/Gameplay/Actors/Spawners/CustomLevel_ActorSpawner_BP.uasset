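; CustomLevel_ActorSpawner_BP is a spawner actor for custom levels that places a given actor class at its own transform.
; Its SpawnActor event stores the class and both block types, always spawns regardless of collision, and records the result as OccupyingActor.
; If that actor is a Destructible_BP or Indestructible_BP, it passes on the matching type through MCSetDestructible or MCSetIndestructible to set the mesh.
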(event Custom|SpawnActor
  (params (Class :type Actor%20Class%20Reference) (Destructible_Type :type Destructible_Types%20Enum :default "NewEnumerator0") (Indestructible_Type :type Indestructible_Types%20Enum :default "NewEnumerator0"))
  (Variables|Default|SetClass Class)
  (Variables|Default|SetDestructible_Type Destructible_Type)
  (Variables|Default|SetIndestructible_Type Indestructible_Type)
  (bind _returnvalue (Game|SpawnActorfromClass (Variables|Default|GetClass) (Transformation|GetActorTransform) "AlwaysSpawn" 0 0))
  (bind _output_get (Variables|Default|SetOccupyingActor _returnvalue))
  ;[0.1979 0.1979 0.1979] Check if the 'Occupying Actor' is of the class 'Destructible_BP' or 'Indestructible_BP'. If true, then set the corresponding selected Mesh type on the actor.
  (bind _asdestructible_bp (Utilities|Casting|CastToDestructible_BP _output_get)
    (:then
      (Default|MCSetDestructible _asdestructible_bp (Variables|Default|GetDestructible_Type)))
    (:CastFailed
      (bind _asindestructible_bp (Utilities|Casting|CastToIndestructible_BP _output_get))
      (Default|MCSetIndestructible _asindestructible_bp (Variables|Default|GetIndestructible_Type)))))

(fn ConstructionScript)