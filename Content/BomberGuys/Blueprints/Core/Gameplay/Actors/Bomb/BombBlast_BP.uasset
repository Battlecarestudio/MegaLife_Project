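; Bomb blast actor that travels forward up to a blast length, damaging players and destructibles along the way.
; On initiation it turns on particles and repeats a forward box trace every 0.1 seconds, shortening its length on blocking hits and sending interface damage messages to hit actors.
; Tick activates projectile movement once tracing allows it, stops at the blast length, then fades the particles before destroying the actor.
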(event Custom|SR_Initiate_BombBlast
  (params (BlastLength :type Float%20%28single-precision%29))
  ;[0.1979 0.1979 0.1979] Traces for conflicting objects that might stop the Blast from spreading. (Such as walls and Indestructible blocks). If a conflicting object is found in the trace, then then Blast Length gets adjusted accordingly.
  ;
  ; We also attempt to send a Damage Message to any hit actor that implements the Gameplay_Interface. In this game this will succeed for Players and Destructibles
  (CallFunction|MCParticleVisibility 3e+02) ; Sets the particle spawn rate\n\nBasically activates the particle
  (Variables|Default|SetBlastLength BlastLength)
  (Variables|Default|SetStartLocation (Transformation|GetActorLocation))
  (bind (_outhits _returnvalue) (Class|KismetSystemLibrary|BoxTraceMulti (Variables|Default|GetStartLocation) (+ (Variables|Default|GetStartLocation) (* (Transformation|GetActorForwardVector) (Variables|Default|GetBlastLength))) "40.000000,40.000000,40.000000" "0, 0, 0" "TraceTypeQuery1" false 0 "None" true))
  (for _array_element _outhits
    (if _returnvalue
      (Variables|Default|SetBlastLength (.Distance (Collision|BreakHitResult _array_element))))
    (Variables|Default|SetCanMove? true)
    ;;[1 1 1 1 14] Triggers the damage event on any actor hit that has the Gameplay_Interace implemented. (PlayerCharacters and Destructibles)
    (Class|GameplayInterface|Damage(Message) (.HitActor (Collision|BreakHitResult _array_element))))
  (Variables|Default|SetCanMove? true)
  ;;[1 1 1] We trace every .1 seconds untill this Blast Actor gets destroyed
  (Utilities|FlowControl|Delay 0.1)
  (CallFunction|Repeat))

(event Custom|Repeat
  (bind _startlocation (Variables|Default|GetStartLocation))
  ;[0.1979 0.1979 0.1979] Traces for conflicting objects that might stop the Blast from spreading. (Such as walls and Indestructible blocks). If a conflicting object is found in the trace, then then Blast Length gets adjusted accordingly.
  ;
  ; We also attempt to send a Damage Message to any hit actor that implements the Gameplay_Interface. In this game this will succeed for Players and Destructibles
  (bind (_outhits _returnvalue) (Class|KismetSystemLibrary|BoxTraceMulti _startlocation (+ _startlocation (* (Transformation|GetActorForwardVector) (Variables|Default|GetBlastLength))) "40.000000,40.000000,40.000000" "0, 0, 0" "TraceTypeQuery1" false 0 "None" true))
  (for _array_element _outhits
    (if _returnvalue
      (Variables|Default|SetBlastLength (.Distance (Collision|BreakHitResult _array_element))))
    (Variables|Default|SetCanMove? true)
    ;;[1 1 1 1 14] Triggers the damage event on any actor hit that has the Gameplay_Interace implemented. (PlayerCharacters and Destructibles)
    (Class|GameplayInterface|Damage(Message) (.HitActor (Collision|BreakHitResult _array_element))))
  (Variables|Default|SetCanMove? true)
  ;;[1 1 1] We trace every .1 seconds untill this Blast Actor gets destroyed
  (Utilities|FlowControl|Delay 0.1)
  (CallFunction|Repeat))

(event Custom|MC_Particle_Visibility
  (params (ParticleSpawnRate :type Float%20%28single-precision%29))
  ;[0.1979 0.1979 0.1979] Traces for conflicting objects that might stop the Blast from spreading. (Such as walls and Indestructible blocks). If a conflicting object is found in the trace, then then Blast Length gets adjusted accordingly.
  ;
  ; We also attempt to send a Damage Message to any hit actor that implements the Gameplay_Interface. In this game this will succeed for Players and Destructibles
  (Effects|Components|ParticleSystem|SetFloatParameter (Variables|Default|GetBlastParticle) "ParticleSpawnRate" ParticleSpawnRate))

(event EventTick
  (params (DeltaSeconds :type Float%20%28single-precision%29))
  ;[0.1979 0.1979 0.1979] Activates the projectile component as soo as [CanMove?] returns true. Stops it's movement as soon as [Stop?] returns true
  (if (Variables|Default|GetCanMove?)
    (Utilities|FlowControl|Sequence
      (:then_0
        (if (Variables|Default|GetStop?)
          (Components|Movement|StopMovementImmediately (Variables|Default|GetProjectileMovement))
          (else
            ;[0.1979 0.1979 0.1979] Checks if explosion travelled a distance >= [BlastLength], if true, stops Blast from going forward > Stops particles > Destroys entire Actor
            (if (>= (Math|Vector|VectorLength (- (Variables|Default|GetStartLocation) (Transformation|GetActorLocation))) (Variables|Default|GetBlastLength))
              (Variables|Default|SetStop? true)
              ;;[1 1 1] Spawns Particles for [0.1] more seconds in-place once explosion reached destination
              (Utilities|FlowControl|Delay 0.1)
              ;;[1 1 1] Afterwards sets [ParticleSpawnRate] of particle to 0 so that no new Blast particles get created
              (Effects|Components|ParticleSystem|SetFloatParameter (Variables|Default|GetBlastParticle) "ParticleSpawnRate" 0.0)
              ;;[1 1 1] After the Particle's Lifetime we destroy the Actor. (So make sure that the Delay Duration before we call Destroy Actor is equal or bigger than the Particles Lifetime.)
              (Utilities|FlowControl|Delay 0.7)
              (Actor|DestroyActor)))))
      (:then_1
        (Utilities|FlowControl|DoOnce false
          (:Completed
            (Components|Activation|Activate (Variables|Default|GetProjectileMovement) false)))))))

(fn ConstructionScript
  (Effects|Components|ParticleSystem|SetFloatParameter (Variables|Default|GetBlastParticle) "ParticleSpawnRate" 0.0))