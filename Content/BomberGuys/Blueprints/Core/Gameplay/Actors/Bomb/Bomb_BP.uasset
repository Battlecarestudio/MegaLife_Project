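; Networked bomb that players drop, which explodes when its fuse timeline ends or shortly after taking damage from another blast.
; Ignition pre-spawns four directional BombBlast_BP actors so particles appear in sync, while a timeline animates glow and size.
; Exploding triggers those blasts, frees the spawner and refunds the owner's bomb.
; Players overlapping at spawn ignore bomb collision via multicast until they leave its overlap volume.
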(event OnComponentEndOverlap(BombOverlapCollision)
  (params (OverlappedComponent :type Primitive%20Component%20Object%20Reference) (OtherActor :type Actor%20Object%20Reference) (OtherComp :type Primitive%20Component%20Object%20Reference) (OtherBodyIndex :type Integer))
  ;[0.1979 0.1979 0.1979] Handle Bomb collissions
  ;;[1 1 1] 3. When a player at some point does leave the bombs location, and thus exits the bomb, then at that point we reset his/hers collision with the bomb so the he/she does also now collide with the bomb
  (Networking|SwitchHasAuthority
    (:Authority
      (CallFunction|MCResetCollisionOverlappingActor OtherActor))))

(event Custom|Explode
  ;[0.1979 0.1979 0.1979] Explode
  ;;[1 1 1] Sets Visibility Collision Response channel to ignore so that the blast can't hit the bomb, and Initiates the pre-spawned blasts
  (Variables|Default|SetExploded? true)
  (Collision|SetCollisionResponsetoChannel (Variables|Default|GetBombOverlapCollision) "ECC_Visibility" "ECR_Ignore")
  (for _array_element (Variables|Default|GetSpawnedBlasts)
    (Default|SRInitiateBombBlast _array_element (Variables|Default|GetBlast%20Length)))
  ;;[1 1 1 1 14] gives the character that dropped this bomb a bomb back
  (bind _asgameplay_character (Utilities|Casting|CastToGameplay_Character (Variables|Default|GetBomb_Owner))
    (:then
      (Math|Integer|IncrementInt (Variables|/Game/BomberGuys/Blueprints/Core/Gameplay/Gameplay_Character.Gameplay_Character_C|GetAmoutOfBombs_Ready _asgameplay_character)
        (:%20%20
          _)))
    (:CastFailed
      _))
  (Actor|DestroyActor))

(event Custom|MC_IgniteBomb
  (params (ActorSpawner :type Bomb%20Spawner%20BP%20Object%20Reference) (BlastLength :type Float%20%28single-precision%29) (Owner :type Actor%20Object%20Reference))
  ;[0.1979 0.1979 0.1979] Spawns a Bomb Ignition sound
  (bind _returnvalue (Audio|SpawnSoundatLocation "/Game/BomberGuys/Assets/Audio/Files/SFX/FireSizzleSparkler_Cue.FireSizzleSparkler_Cue" (Transformation|GetActorLocation) "0, 0, 0" 0.7 1.0 0.0 0 0))
  (Variables|Default|SetActiveSound _returnvalue)
  (Networking|SwitchHasAuthority
    (:Authority
      (CallFunction|SpawnBlasts)
      (Variables|Default|SetActorSpawner ActorSpawner)
      (Variables|Default|SetBlast%20Length BlastLength)
      (Variables|Default|SetBomb_Owner Owner)
      ;[0.1979 0.1979 0.1979 1 12] Sets the ActorSpawner to be occupied
      (Variables|/Game/BomberGuys/Blueprints/Core/Gameplay/Actors/Spawners/BombSpawner_BP.BombSpawner_BP_C|SetOccupied? (Variables|Default|GetActorSpawner) true)
      ;[0.1979 0.1979 0.1979] Changes color / size of bomb for 3 seconds to indicate that the explosion is coming
      (bind (_direction _emissivecolor _bombsize) (Timeline|Emissive/Scale_Change PlayFromStart)
        (:Update
          (Rendering|Material|SetScalarParameterValueonMaterials (Variables|Default|GetBomb_StaticMesh) "Emissive" _emissivecolor)
          (Transformation|SetWorldScale3D (Variables|Default|GetBomb_StaticMesh) (Math|Vector|MakeVector _bombsize _bombsize _bombsize)))
        (:Finished
          ;[0.1979 0.1979 0.1979] Explode once the bomb is done infusing
          (Networking|SwitchHasAuthority
            (:Authority
              (CallFunction|MCExplosionSound)
              (if (not (Variables|Default|GetExploded?))
                ;;[0.1979 0.1979 0.1979 1 12] Sets the ActorSpawner to be unoccupied again
                (Variables|/Game/BomberGuys/Blueprints/Core/Gameplay/Actors/Spawners/BombSpawner_BP.BombSpawner_BP_C|SetOccupied? (Variables|Default|GetActorSpawner) false)
                (CallFunction|Explode)))))))
    (:Remote
      (Timeline|Emissive/Scale_Change PlayFromStart))))

(event Custom|MC_SetCollision_ActorsToIgnore
  ;[0.1979 0.1979 0.1979] Handle Bomb collissions
  ;;[1 1 1] 2. This multicast then sets the collision on all players that have been added to the  [ActorsToIgnore]  array to ignore collision and afterwards turns on its own bomb collision so that the other players that weren't added to this [ActorsToignore] array will collide with this bomb.
  (for _array_element (Variables|Default|GetActorsToIgnore)
    (bind _asgameplay_character (Utilities|Casting|CastToGameplay_Character _array_element))
    (Collision|SetCollisionResponsetoChannel (Variables|/Script/Engine.Character|GetCapsuleComponent _asgameplay_character) "ECC_GameTraceChannel2" "ECR_Ignore"))
  (Collision|SetCollisionEnabled (Variables|Default|GetBombCollision) "QueryAndPhysics"))

(event Custom|MC_ResetCollision_OverlappingActor
  (params (OtherActor :type Object%20Object%20Reference))
  ;[0.1979 0.1979 0.1979] Handle Bomb collissions
  ;;[1 1 1] Resets Collision for whoever left the BombOverlapCollision as explained on the left
  (bind _asgameplay_character (Utilities|Casting|CastToGameplay_Character OtherActor))
  (Collision|SetCollisionResponsetoChannel (Variables|/Script/Engine.Character|GetCapsuleComponent _asgameplay_character) "ECC_GameTraceChannel2" "ECR_Block"))

(event Custom|MC_ExplosionSound
  ;[0.1979 0.1979 0.1979] Multicast: Stops previously spawned ignition sound > Plays Explosion sound
  (bind _activesound (Variables|Default|GetActiveSound)
    (:then
      (Audio|Components|Audio|Stop _activesound))
    (:else
      _))
  (Audio|PlaySoundatLocation "/Game/BomberGuys/Assets/Audio/Files/SFX/Explosion_Cue.Explosion_Cue" (Transformation|GetActorLocation) "0, 0, 0" 1.0 1.0 0.0 0 0 0))

(event EventBeginPlay
  (bind _returnvalue (Transformation|GetActorLocation))
  (bind _returnvalue_2 (+ (.z _returnvalue) 5e+01))
  ;[0.1979 0.1979 0.1979] Handle Bomb collissions
  ;;[1 1 1] 1. When this actor (this bomb) gets spawned into the world, then the Beginplay event fires off a MultiBoxTrace which detects which players were in the bomb upon the bomb being spawned. Those that were get added to the actor to ignore. Once this MultiboxTrace check completed we fire off MC_Set_Collision_ActorsToIgnore
  (Networking|SwitchHasAuthority
    (:Authority
      (bind _outhits (Class|KismetSystemLibrary|BoxTraceMulti (Math|Vector|MakeVector (.x _returnvalue) (.y _returnvalue) _returnvalue_2) (Math|Vector|MakeVector (.x _returnvalue) (.y _returnvalue) _returnvalue_2) "45.000000,45.000000,45.000000" "0, 0, 0" "TraceTypeQuery1" false 0 "None" true "(R=0.000000,G=1.000000,B=0.022676,A=1.000000)"))
      (for _array_element _outhits
        (Utilities|Array|AddUnique (Variables|Default|GetActorsToIgnore) (.HitActor (Collision|BreakHitResult _array_element))))
      (CallFunction|MCSetCollisionActorstoIgnore))))

(event EventDamage
  ;[0.1979 0.1979 0.1979] Explode in case another bomb's blast hit this bomb
  (Utilities|FlowControl|Delay 0.1) ; Delay till bomb explosion because instant doesn't look good
  ;[0.1979 0.1979 0.1979] Explode once the bomb is done infusing
  (Networking|SwitchHasAuthority
    (:Authority
      (CallFunction|MCExplosionSound)
      (if (not (Variables|Default|GetExploded?))
        ;;[0.1979 0.1979 0.1979 1 12] Sets the ActorSpawner to be unoccupied again
        (Variables|/Game/BomberGuys/Blueprints/Core/Gameplay/Actors/Spawners/BombSpawner_BP.BombSpawner_BP_C|SetOccupied? (Variables|Default|GetActorSpawner) false)
        (CallFunction|Explode)))))

(fn ConstructionScript)

(fn SpawnBlasts
  (bind _returnvalue (Transformation|GetActorLocation))
  ;[0.1979 0.1979 0.1979] Spawns a BombBlast_BP in 4 directions (x, x-, y, y-) and adds them to the array of [SpawnedBlasts]
  ;
  ; It's necessary that we pre-spawn these, since when the actor initializes (BombBlast_BP actor) the particle system takes a bit longer to initiate. Hence we pre-spawn these blasts so that once we set the particle to appear, it's visible to all players at the same time.
  (for _array_element (Utilities|Array|MakeArray "1.000000,0.000000,0.000000" "0.000000,1.000000,0.000000" "-1.000000,0.000000,0.000000" "0.000000,-1.000000,0.000000")
    (bind _returnvalue_2 (Game|SpawnActorfromClass "/Game/BomberGuys/Blueprints/Core/Gameplay/Actors/Bomb/BombBlast_BP.BombBlast_BP_C" (Math|Transform|MakeTransform (Math|Vector|MakeVector (.x _returnvalue) (.y _returnvalue) (+ (.z _returnvalue) 5e+01)) (Math|Conversions|RotationFromXVector _array_element) "1,1,1") "AlwaysSpawn" 0 0))
    (Utilities|Array|Add (Variables|Default|GetSpawnedBlasts) _returnvalue_2)))