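; Blueprint function library for BomberGuys that gathers shared helpers for game framework access, UI screens, saving and menu selection.
; Getters return the cast game instance, lobby and gameplay modes, and gameplay state.
; UI helpers spawn fade, loading, transition and error widgets on player 0, including a fade-in that travels to a level.
; Profile and settings helpers use the GameInstance's save object, writing to one general slot, while Switch_Selection steps an index within bounds.
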(fn GetGameInstance
  (bind _asbomber_guys_game_instance (Utilities|Casting|CastToBomberGuys_GameInstance (Game|GetGameInstance)))
  (return _asbomber_guys_game_instance))

(fn GetLobbyGameMode
  (bind _aslobby_game_mode (Utilities|Casting|CastToLobby_GameMode (Game|GetGameMode)))
  (return _aslobby_game_mode))

(fn GetGameplayGameMode
  (bind _asgameplay_game_mode (Utilities|Casting|CastToGameplay_GameMode (Game|GetGameMode)))
  (return _asgameplay_game_mode))

(fn GetGameplayGameState
  (bind _asgameplay_game_state (Utilities|Casting|CastToGameplay_GameState (Game|GetGameState)))
  (return _asgameplay_game_state))

(fn OpenLevelFadeinTransitionScreen
  (params (LevelName :type Name) (Options :type String))
  (bind _returnvalue (Game|GetPlayerController 0))
  (Utilities|IsValid _returnvalue
    (:Is%20Valid
      (if (Pawn|IsLocalPlayerController _returnvalue)
        (bind _returnvalue_2 (UserInterface|CreateWidget "/Game/BomberGuys/Widgets/LoadingScreens/Transition_Fade_Screen_WB.Transition_Fade_Screen_WB_C" _returnvalue))
        (UserInterface|Viewport|AddtoViewport _returnvalue_2 0)
        (Default|FadeinTravel _returnvalue_2 LevelName Options)))))

(fn FadeOutTransitionScreen
  (bind _returnvalue (UserInterface|CreateWidget "/Game/BomberGuys/Widgets/LoadingScreens/Transition_Fade_Screen_WB.Transition_Fade_Screen_WB_C" (Game|GetPlayerController 0)))
  (UserInterface|Viewport|AddtoViewport _returnvalue 0)
  (Default|FadeOut _returnvalue))

(fn FadeinTransitionScreen
  (bind _returnvalue (UserInterface|CreateWidget "/Game/BomberGuys/Widgets/LoadingScreens/Transition_Fade_Screen_WB.Transition_Fade_Screen_WB_C" (Game|GetPlayerController 0)))
  (UserInterface|Viewport|AddtoViewport _returnvalue 0)
  (Default|Fadein _returnvalue))

(fn CreateErrorPopUp
  (params (Error_Message :type String))
  (bind _errorpopup_wb (LocalVariables|GetErrorPopUp_WB)
    (:then
      (if (not (UserInterface|Viewport|IsinViewport _errorpopup_wb))
        (UserInterface|Viewport|AddtoViewport _errorpopup_wb 0 :!label _label)))
    (:else
      (bind _returnvalue (UserInterface|CreateWidget "/Game/BomberGuys/Widgets/General/Error_WB.Error_WB_C" (Game|GetPlayerController 0) Error_Message))
      (LocalVariables|SetErrorPopUp_WB _returnvalue)
      (goto _label))))

(fn CreateLoadingScreen
  (params (LoadingScreen_Text :type Text))
  (bind _returnvalue (UserInterface|CreateWidget "/Game/BomberGuys/Widgets/LoadingScreens/LoadingScreen_WB.LoadingScreen_WB_C" (Game|GetPlayerController 0)))
  (UserInterface|Viewport|AddtoViewport _returnvalue 0)
  (Default|Initialize _returnvalue LoadingScreen_Text))

(fn CreateTransitionScreen
  (params (EnteringGameText_Vis :type ESlateVisibility%20Enum :default "Visible"))
  (bind _returnvalue (UserInterface|CreateWidget "/Game/BomberGuys/Widgets/LoadingScreens/TransitionScreen_WB.TransitionScreen_WB_C" (Game|GetPlayerController 0) EnteringGameText_Vis))
  (UserInterface|Viewport|AddtoViewport _returnvalue 0))

(fn FadeIn/OutAnimation
  (bind _returnvalue (UserInterface|CreateWidget "/Game/BomberGuys/Widgets/LoadingScreens/Transition_Fade_Screen_WB.Transition_Fade_Screen_WB_C" (Game|GetPlayerController 0)))
  (UserInterface|Viewport|AddtoViewport _returnvalue 0)
  (Default|FadeIn/Out _returnvalue))

(fn GetAllLevelNames
  (return (LocalVariables|GetLevelNames)))

(fn SavePlayerProfile
  (params (PlayerProfile :type User%20Profile%20Structure%20Structure))
  (bind _asbomber_guy_game_instance (Casts|GetGameInstance))
  (bind _general_savegameobject (Variables|/Game/BomberGuys/Blueprints/GameInstance/BomberGuys_GameInstance.BomberGuys_GameInstance_C|GetGeneral_SaveGameObject _asbomber_guy_game_instance))
  (Variables|/Game/BomberGuys/Blueprints/SaveGames/General_SaveGame.General_SaveGame_C|SetPlayerProfile _general_savegameobject PlayerProfile)
  (SaveGame|SaveGametoSlot _general_savegameobject "General_SaveSlot")
  (return))

(fn SwitchSelection
  (params (Current_Selection :type Integer) (Minimum_Options :type Integer) (Max_Options :type Integer) (Decrease? :type Boolean))
  (LocalVariables|SetCurrentSelection Current_Selection)
  (LocalVariables|SetMinimumSelection Minimum_Options)
  (LocalVariables|SetMaxSelection Max_Options)
  (if Decrease?
    (if (<= (LocalVariables|GetCurrentSelection) (LocalVariables|GetMinimumSelection))
      (LocalVariables|SetCurrentSelection (LocalVariables|GetMinimumSelection))
      (else
        (Math|Integer|DecrementInt (LocalVariables|GetCurrentSelection)
          (:%20%20
            _))))
    (elif (>= (LocalVariables|GetCurrentSelection) (LocalVariables|GetMaxSelection))
      (LocalVariables|SetCurrentSelection (LocalVariables|GetMaxSelection))
      (else
        (Math|Integer|IncrementInt (LocalVariables|GetCurrentSelection)
          (:%20%20
            _)))))
  (return (LocalVariables|GetCurrentSelection)))

(fn SaveGameSettings
  (params (GameSettings :type Game%20Settings%20Structure%20Structure))
  (bind _asbomber_guy_game_instance (Casts|GetGameInstance))
  (bind _general_savegameobject (Variables|/Game/BomberGuys/Blueprints/GameInstance/BomberGuys_GameInstance.BomberGuys_GameInstance_C|GetGeneral_SaveGameObject _asbomber_guy_game_instance))
  (Variables|/Game/BomberGuys/Blueprints/SaveGames/General_SaveGame.General_SaveGame_C|SetGameSettings _general_savegameobject GameSettings)
  (SaveGame|SaveGametoSlot _general_savegameobject "General_SaveSlot"))

(fn GetGameSettings
  (return (Variables|/Game/BomberGuys/Blueprints/SaveGames/General_SaveGame.General_SaveGame_C|GetGameSettings (Variables|/Game/BomberGuys/Blueprints/GameInstance/BomberGuys_GameInstance.BomberGuys_GameInstance_C|GetGeneral_SaveGameObject (Casts|GetGameInstance)))))

(fn GetPlayerProfile
  (return (Variables|/Game/BomberGuys/Blueprints/SaveGames/General_SaveGame.General_SaveGame_C|GetPlayerProfile (Variables|/Game/BomberGuys/Blueprints/GameInstance/BomberGuys_GameInstance.BomberGuys_GameInstance_C|GetGeneral_SaveGameObject (Casts|GetGameInstance)))))