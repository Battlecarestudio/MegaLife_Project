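; Main menu display actor that spins a mesh and periodically swaps it for a random block, prop or item from the game.
; A looping RotateSwitch timeline drives the mesh yaw and picks a new mesh each time it finishes.
; The SameAsLast macro rerolls recursively on a repeat, otherwise applies the mesh with a standard or adjusted transform, and a poof particle spawns on each swap.
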(event Custom|Rotate/Switch_Cube
  ;[0.1979 0.1979 0.1979] Rotates and switches out the actors mesh every x seconds.
  ;
  ; This actor is used in the MainMenu
  (bind _rotate (Timeline|Rotate/Switch PlayFromStart)
    (:Update
      (Transformation|SetRelativeRotation (Variables|Default|GetStaticMesh) (Math|Rotator|MakeRotator 0.0 0.0 _rotate) false false))
    (:Finished
      (CallFunction|ChooseNewMesh)
      (CallFunction|Rotate/SwitchCube))))

(event EventBeginPlay
  ;[0.1979 0.1979 0.1979] Rotates and switches out the actors mesh every x seconds.
  ;
  ; This actor is used in the MainMenu
  (CallFunction|Rotate/SwitchCube)
  (CallFunction|ChooseNewMesh))

(fn ConstructionScript)

(fn ChooseNewMesh
  ;[0.1979 0.1979 0.1979] Randomly selects a new mesh and sets it
  (switch int (Math|Random|RandomIntegerinRange 0 13)
    (:0
      (Utilities|SameasLast? "/Game/BomberGuys/Assets/3D_Assets/Meshes/Blocks/Books_Indestructible.Books_Indestructible" false
        (:New
          _)))
    (:1
      (Utilities|SameasLast? "/Game/BomberGuys/Assets/3D_Assets/Meshes/Blocks/Bricks_Destructible.Bricks_Destructible" false
        (:New
          _)))
    (:2
      (Utilities|SameasLast? "/Game/BomberGuys/Assets/3D_Assets/Meshes/Blocks/ConstructionBlock_Indestructible.ConstructionBlock_Indestructible" false
        (:New
          _)))
    (:3
      (Utilities|SameasLast? "/Game/BomberGuys/Assets/3D_Assets/Meshes/Blocks/MetalBlock_Indestructible.MetalBlock_Indestructible" false
        (:New
          _)))
    (:4
      (Utilities|SameasLast? "/Game/BomberGuys/Assets/3D_Assets/Meshes/Blocks/MetalPipes_Destructible.MetalPipes_Destructible" false
        (:New
          _)))
    (:5
      (Utilities|SameasLast? "/Game/BomberGuys/Assets/3D_Assets/Meshes/Blocks/MovingBox_Destructible.MovingBox_Destructible" false
        (:New
          _)))
    (:6
      (Utilities|SameasLast? "/Game/BomberGuys/Assets/3D_Assets/Meshes/Blocks/NeonCube_Destructible.NeonCube_Destructible" false
        (:New
          _)))
    (:7
      (Utilities|SameasLast? "/Game/BomberGuys/Assets/3D_Assets/Meshes/Blocks/TreeGreen_Destructible.TreeGreen_Destructible" false
        (:New
          _)))
    (:8
      (Utilities|SameasLast? "/Game/BomberGuys/Assets/3D_Assets/Meshes/SpawnFlag/CustomLevel_PlayerSpawn.CustomLevel_PlayerSpawn" false
        (:New
          _)))
    (:9
      (Utilities|SameasLast? "/Game/BomberGuys/Assets/3D_Assets/Meshes/Props/DogHouse_Prop.DogHouse_Prop" false
        (:New
          _)))
    (:10
      (Utilities|SameasLast? "/Game/BomberGuys/Assets/3D_Assets/Meshes/Props/Dumpster_Green_Prop.Dumpster_Green_Prop" false
        (:New
          _)))
    (:11
      (Utilities|SameasLast? "/Game/BomberGuys/Assets/3D_Assets/Meshes/Items/SpeedDown.SpeedDown" true
        (:New
          _)))
    (:12
      (Utilities|SameasLast? "/Game/BomberGuys/Assets/3D_Assets/Meshes/Items/SpeedUp_Item.SpeedUp_Item" true
        (:New
          _)))
    (:13
      (Utilities|SameasLast? "/Game/BomberGuys/Assets/3D_Assets/Meshes/Items/FireUp_Item.FireUp_Item" true
        (:New
          _))))
  (Niagara|SpawnSystematLocation "/Game/BomberGuys/Assets/Niagara_Particles/Poof/Poof_Particle.Poof_Particle" (Transformation|GetWorldLocation (Variables|Default|GetStaticMesh)) "0, 0, 0" "3.000000,3.000000,3.000000")
  (return))