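; Base_NeonCube_BP is a decorative neon cube actor that animates its NeonCube component with a preset motion.
; On BeginPlay it switches on the MovementMethod setting to pick Z spin, all-axis spin, vertical or sideways movement, or a combined spin and bob.
; Each motion is driven by a Timeline that writes the component's relative rotation or location, with the combined mode reusing the Z spin alongside its own vertical timeline.
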(event EventBeginPlay
  (switch Utilities|FlowControl|Switch|SwitchonNeonCube_Enum (Variables|Default|GetMovementMethod)
    (:NewEnumerator0
      (bind _rotate (Timeline|RotateZ Play)
        (:Update
          (Transformation|SetRelativeRotation (Variables|Default|GetNeonCube) (Math|Rotator|MakeRotator 0.0 0.0 _rotate) false false))))
    (:NewEnumerator1
      (bind _rotate_2 (Timeline|RotateXYZ Play)
        (:Update
          (Transformation|SetRelativeRotation (Variables|Default|GetNeonCube) (Math|Rotator|MakeRotator _rotate_2 _rotate_2 _rotate_2) false false))))
    (:NewEnumerator2
      (bind _updown (Timeline|UpDown Play)
        (:Update
          (Transformation|SetRelativeLocation (Variables|Default|GetNeonCube) (Math|Vector|MakeVector 0.0 0.0 _updown) false false))))
    (:NewEnumerator3
      (bind _leftright (Timeline|LeftRight Play)
        (:Update
          (Transformation|SetRelativeLocation (Variables|Default|GetNeonCube) (Math|Vector|MakeVector 0.0 _leftright 0.0) false false))))
    (:NewEnumerator4
      (Utilities|FlowControl|Sequence
        (:then_0
          (Timeline|RotateZ Play))
        (:then_1
          (bind _updown_2 (Timeline|UpDownCombo Play)
            (:Update
              (Transformation|SetRelativeLocation (Variables|Default|GetNeonCube) (Math|Vector|MakeVector 0.0 0.0 _updown_2) false false))))))))

(fn ConstructionScript)