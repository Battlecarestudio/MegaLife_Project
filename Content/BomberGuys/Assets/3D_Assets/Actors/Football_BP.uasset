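; Football actor that Lobby_Character players can hit, respawning itself whenever it reaches the goal.
; Tick compares its position to GoalLocation within a tolerance, then once plays the goal sound, spawns a replacement ball at a hard-coded point with the same GoalLocation, and destroys itself.
; Sphere overlaps with a Lobby_Character play a hit sound, throttled by a flag and short delay.
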(event OnComponentBeginOverlap(Sphere)
  (params (OverlappedComponent :type Primitive%20Component%20Object%20Reference) (OtherActor :type Actor%20Object%20Reference) (OtherComp :type Primitive%20Component%20Object%20Reference) (OtherBodyIndex :type Integer) (bFromSweep :type Boolean) (SweepResult :type Hit%20Result%20Structure%20%28by%20ref%29))
  ;[1 1 1] Plays a sound when the players hits the ball
  (Utilities|Casting|CastToLobby_Character OtherActor)
  (if (Variables|Default|GetReadyToPlaySound?)
    (Audio|PlaySoundatLocation "/Game/BomberGuys/Assets/Audio/Files/SFX/SoccerBall_Cue.SoccerBall_Cue" (Transformation|GetActorLocation) "0, 0, 0" 1.0 1.0 0.0 0 0 0)
    (Variables|Default|SetReadyToPlaySound? false)
    (Utilities|FlowControl|Delay 0.5)
    (Variables|Default|SetReadyToPlaySound? true)))

(event EventTick
  (params (DeltaSeconds :type Float%20%28single-precision%29))
  ;[1 1 1] When the soccerball's location is equal to the goal location then we spawn another soccerbal and destroy this one
  (if (Math|Vector|Equal(Vector) (Variables|Default|GetGoalLocation) (Transformation|GetActorLocation) 8e+01)
    (Utilities|FlowControl|DoOnce false
      (:Completed
        (Audio|PlaySoundatLocation "/Game/BomberGuys/Assets/Audio/Files/SFX/GoalScore_Cue.GoalScore_Cue" (Transformation|GetActorLocation) "0, 0, 0" 1.0 1.0 0.0 0 0 0)
        (Game|SpawnActorfromClass "Football_BP_C" (Math|Transform|MakeTransform "-630.000000,-490.000000,250.000000") "Undefined" 0 (Variables|Default|GetGoalLocation) "0.000000,0.000000,0.000000|0.000000,0.000000,0.000000|1.000000,1.000000,1.000000" 0)
        (Actor|DestroyActor)))))

(fn ConstructionScript)